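; BP_Skeleton is the third-person player character, with camera-relative Enhanced Input movement, jumping and a mid-air dash on a one-second lockout.
; A timeline driven by a FlipFlop blends the spring arm between left and right shoulder views.
; It counts coins, triggers checks on overlapping puzzle gates and opens the pause menu.
; Any damage ragdolls it, then GM_MicroGame, given its spawn transform at BeginPlay, respawns the player after a delay.
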(event Input|EnhancedActionEvents|EnhancedInputActionIA_MoveForward
  (params (ActionValue :type Float%20%28double-precision%29) (ElapsedSeconds :type Float%20%28double-precision%29) (TriggeredSeconds :type Float%20%28double-precision%29) (InputAction :type Input%20Action%20Object%20Reference :default "/Game/MicroGame/Input/IA_MoveForward.IA_MoveForward"))
  (Pawn|Input|AddMovementInput (Math|Vector|GetForwardVector (Math|Rotator|MakeRotator 0.0 0.0 (.Yaw (Math|Rotator|BreakRotator (Pawn|GetControlRotation :!class /Script/Engine.Pawn))))) ActionValue false))

(event Input|EnhancedActionEvents|EnhancedInputActionIA_MoveRight
  (params (ActionValue :type Float%20%28double-precision%29) (ElapsedSeconds :type Float%20%28double-precision%29) (TriggeredSeconds :type Float%20%28double-precision%29) (InputAction :type Input%20Action%20Object%20Reference :default "/Game/MicroGame/Input/IA_MoveRight.IA_MoveRight"))
  (Pawn|Input|AddMovementInput (Math|Vector|GetRightVector (Math|Rotator|MakeRotator 0.0 0.0 (.Yaw (Math|Rotator|BreakRotator (Pawn|GetControlRotation :!class /Script/Engine.Pawn))))) ActionValue false))

(event Input|EnhancedActionEvents|EnhancedInputActionIA_MoveTurn
  (params (ActionValue :type Float%20%28double-precision%29) (ElapsedSeconds :type Float%20%28double-precision%29) (TriggeredSeconds :type Float%20%28double-precision%29) (InputAction :type Input%20Action%20Object%20Reference :default "/Game/MicroGame/Input/IA_MoveTurn.IA_MoveTurn"))
  (Pawn|Input|AddControllerYawInput ActionValue))

(event Input|EnhancedActionEvents|EnhancedInputActionIA_ShoSwitch
  (params (ActionValue :type Boolean) (ElapsedSeconds :type Float%20%28double-precision%29) (TriggeredSeconds :type Float%20%28double-precision%29) (InputAction :type Input%20Action%20Object%20Reference :default "/Game/MicroGame/Input/IA_ShoSwitch.IA_ShoSwitch"))
  (Utilities|FlowControl|FlipFlop
    (:A
      (bind _camlocblendalpha (Timeline|T_ShoSwitch Play)
        (:Update
          (Transformation|SetRelativeLocation (Variables|Default|GetShoulderSpringArm) (Math|Vector|Lerp(Vector) (Variables|Default|GetLShoCamLoc) (Variables|Default|GetRShoCamLoc) _camlocblendalpha) false false))))
    (:B
      (Timeline|T_ShoSwitch Reverse))))

(event Input|EnhancedActionEvents|EnhancedInputActionIA_LookUp
  (params (ActionValue :type Float%20%28double-precision%29) (ElapsedSeconds :type Float%20%28double-precision%29) (TriggeredSeconds :type Float%20%28double-precision%29) (InputAction :type Input%20Action%20Object%20Reference :default "/Game/MicroGame/Input/IA_LookUp.IA_LookUp"))
  (Pawn|Input|AddControllerPitchInput ActionValue))

(event Input|EnhancedActionEvents|EnhancedInputActionIA_Jump
  (params (ActionValue :type Boolean) (ElapsedSeconds :type Float%20%28double-precision%29) (TriggeredSeconds :type Float%20%28double-precision%29) (InputAction :type Input%20Action%20Object%20Reference :default "/Game/MicroGame/Input/IA_Jump.IA_Jump"))
  (Character|Jump))

(event Input|EnhancedActionEvents|EnhancedInputActionIA_Pause
  (params (ActionValue :type Boolean) (ElapsedSeconds :type Float%20%28double-precision%29) (TriggeredSeconds :type Float%20%28double-precision%29) (InputAction :type Input%20Action%20Object%20Reference :default "/Game/MicroGame/Input/IA_Pause.IA_Pause"))
  (bind _returnvalue (Game|GetPlayerController 0))
  ;[1 1 1] Pause Game
  (:Started
    (bind _returnvalue_2 (UserInterface|CreateWidget "/Game/MicroGame/UI/PauseMenu_UI.PauseMenu_UI_C"))
    (UserInterface|Viewport|AddtoViewport _returnvalue_2 0)
    (Variables|/Script/Engine.PlayerController|SetbShowMouseCursor _returnvalue true)
    (Input|SetInputModeUIOnly _returnvalue 0 "DoNotLock" false)
    (Game|SetGamePaused true)))

(event Input|EnhancedActionEvents|EnhancedInputActionIA_JumpSound
  (params (ActionValue :type Boolean) (ElapsedSeconds :type Float%20%28double-precision%29) (TriggeredSeconds :type Float%20%28double-precision%29) (InputAction :type Input%20Action%20Object%20Reference :default "/Game/MicroGame/Input/IA_JumpSound.IA_JumpSound"))
  (if (not (AI|Components|NavMovement|IsFalling (Variables|Character|GetCharacterMovement)))
    (Audio|PlaySound2D "/Game/MicroGame/Audio/Jump.Jump" 1.0 1.0 0.0 0 0)))

(event Input|EnhancedActionEvents|EnhancedInputActionIA_Interact
  (params (ActionValue :type Boolean) (ElapsedSeconds :type Float%20%28double-precision%29) (TriggeredSeconds :type Float%20%28double-precision%29) (InputAction :type Input%20Action%20Object%20Reference :default "/Game/MicroGame/Input/IA_Interact.IA_Interact"))
  (for _array_element (Collision|GetOverlappingActors 0 :!class /Script/Engine.Actor)
    (bind _asbp_puzzle_gate (Utilities|Casting|CastToBP_PuzzleGate _array_element))
    (Default|OpenDoorCheck _asbp_puzzle_gate)))

(event Input|EnhancedActionEvents|EnhancedInputActionIA_Dash
  (params (ActionValue :type Boolean) (ElapsedSeconds :type Float%20%28double-precision%29) (TriggeredSeconds :type Float%20%28double-precision%29) (InputAction :type Input%20Action%20Object%20Reference :default "/Game/MicroGame/Input/IA_Dash.IA_Dash"))
  (bind _charactermovement (Variables|Character|GetCharacterMovement))
  (bind _returnvalue (Pawn|Components|PawnMovement|GetLastInputVector _charactermovement))
  (bind _returnvalue_2 (* _returnvalue 5e+03))
  (if (AI|Components|NavMovement|IsFalling (Variables|Character|GetCharacterMovement))
    (if (not (Variables|Default|GetisDashing))
      (Variables|Default|SetisDashing true)
      (Character|LaunchCharacter (Math|Vector|MakeVector (.x _returnvalue_2) (.y _returnvalue_2) 0.0) false false)
      (Utilities|FlowControl|Delay 1.0)
      (Variables|Default|SetisDashing false))))

(event EventBeginPlay
  (bind _asgm_micro_game (Utilities|Casting|CastToGM_MicroGame (Game|GetGameMode)))
  (Variables|/Game/MicroGame/Blueprints/GM_MicroGame.GM_MicroGame_C|SetSpawn%20Transform _asgm_micro_game (Transformation|GetActorTransform)))

(event Collision|EventActorBeginOverlap
  (params (OtherActor :type Actor%20Object%20Reference)))

(event EventTick
  (params (DeltaSeconds :type Float%20%28single-precision%29)))

(event EventPossessed
  (params (NewController :type Controller%20Object%20Reference))
  (bind _asplayer_controller (Utilities|Casting|CastToPlayerController NewController))
  (Input|AddMappingContext (PlayerController|LocalPlayerSubsystems|GetEnhancedInputLocalPlayerSubsystem _asplayer_controller) "/Game/MicroGame/Input/IM_ThirdPerson.IM_ThirdPerson" 0 "(bIgnoreAllPressedKeysUntilRelease=True,bForceImmediately=False,bNotifyUserSettings=False)"))

(event EventOnCoinCollected
  ;[1 1 1] Set Coin Counter
  (Math|Integer|IncrementInt (Variables|Default|GetCurrentCoins)))

(event Game|Damage|EventAnyDamage
  (params (Damage :type Float%20%28single-precision%29) (DamageType :type Damage%20Type%20Object%20Reference) (InstigatedBy :type Controller%20Object%20Reference) (DamageCauser :type Actor%20Object%20Reference))
  (Audio|PlaySound2D "/Game/MicroGame/Audio/DeathBell.DeathBell" 1.0 1.0 0.0 0 0)
  (Physics|SetSimulatePhysics (Variables|Character|GetMesh) true)
  (Input|DisableInput 0)
  (Utilities|FlowControl|Delay 2.0)
  (bind _asgm_micro_game (Utilities|Casting|CastToGM_MicroGame (Game|GetGameMode)))
  (Default|RespawnPlayer _asgm_micro_game))

(fn ConstructionScript
  (Transformation|SetRelativeLocation (Variables|Default|GetShoulderSpringArm) (Variables|Default|GetLShoCamLoc) false false))

(fn GetCoins
  (return (Variables|Default|GetCurrentCoins)))