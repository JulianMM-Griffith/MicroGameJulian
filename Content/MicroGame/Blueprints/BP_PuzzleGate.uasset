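; BP_PuzzleGate is a gate that swings its door open once enough puzzle items have been collected.
; CollectItem increments a counter, while a separate OpenDoorCheck event compares it to the required maximum and fires OpenDoor through a DoOnce.
; OpenDoor plays a timeline that lerps the door's relative yaw to a quarter turn.
; A disconnected node that would slide the door instead is left unused.
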(event Custom|OpenDoor
  (bind _door_rotation (Timeline|Open%20Door%20Animation%20Rotation Play)
    (:Update
      (Transformation|SetRelativeRotation (Variables|Default|GetDoor) (Math|Rotator|MakeRotator 0.0 0.0 (Math|Float|Lerp 0.0 9e+01 _door_rotation)) false false))))

(event Custom|CollectItem
  (Math|Integer|IncrementInt (Variables|Default|GetCurrentItemsCollected)))

(event Custom|Open%20Door%20Check
  (if (>= (Variables|Default|GetCurrentItemsCollected) (Variables|Default|GetMaxItemsCollected))
    (Utilities|FlowControl|DoOnce false
      (:Completed
        (CallFunction|OpenDoor)))))

(fn ConstructionScript)