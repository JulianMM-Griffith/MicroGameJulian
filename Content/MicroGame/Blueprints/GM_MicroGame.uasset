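; GM_MicroGame is the micro game's game mode Blueprint, handling player respawn through a RespawnPlayer event.
; The event destroys the current player character, then spawns a fresh BP_Skeleton at the LastCheckpoint's POS transform, or at the default transform if no checkpoint is valid.
; Player controller 0 then possesses the new skeleton, and spawning always succeeds regardless of collision.
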(event Custom|RespawnPlayer
  (Actor|DestroyActor (Game|GetPlayerCharacter 0))
  (bind _lastcheckpoint (Variables|Default|GetlastCheckpoint)
    (:then
      (bind _returnvalue (Game|SpawnActorfromClass "/Game/MicroGame/Blueprints/BP_Skeleton.BP_Skeleton_C" (Math|Transform|MakeTransform (.location (Transformation|GetWorldTransform (Variables|/Game/MicroGame/Blueprints/BP_Checkpoint.BP_Checkpoint_C|GetPOS _lastcheckpoint))) (.rotation (Transformation|GetWorldTransform (Variables|/Game/MicroGame/Blueprints/BP_Checkpoint.BP_Checkpoint_C|GetPOS _lastcheckpoint))) (.scale (Transformation|GetWorldTransform (Variables|/Game/MicroGame/Blueprints/BP_Checkpoint.BP_Checkpoint_C|GetPOS _lastcheckpoint)))) "AlwaysSpawn" "MultiplyWithRoot" 0 0))
      (Pawn|Possess (Game|GetPlayerController 0) _returnvalue))
    (:else
      (bind _returnvalue_2 (Game|SpawnActorfromClass "/Game/MicroGame/Blueprints/BP_Skeleton.BP_Skeleton_C" (Math|Transform|MakeTransform "0, 0, 0" "0, 0, 0" "1.000000,1.000000,1.000000") "AlwaysSpawn" "MultiplyWithRoot" 0 0))
      (Pawn|Possess (Game|GetPlayerController 0) _returnvalue_2))))

(event EventBeginPlay)

(event EventTick
  (params (DeltaSeconds :type Float%20%28single-precision%29)))

(fn ConstructionScript)